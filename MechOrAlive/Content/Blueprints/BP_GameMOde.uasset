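; Game mode for a two-team ball game with mechs, handling cameras, scoring, resets and the win announcement.
; BeginPlay finds the play and menu cameras, views through the menu camera, adds the GameUI widget and hides the win display.
; IncreaseScore awards a point on a team's second consecutive bounce, then resets ball and mechs with a brief music switch.
; Reaching MaxScore sets the winner text, reveals BP_Win and changes the music.
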(event Custom|IncreaseScore
  (params (Team :type Integer))
  (Variables|Default|SetTempTeam Team)
  (if (>= (Utilities|Array|Get(acopy) (Variables|Default|GetBounces) (Variables|Default|GetTempTeam)) 1)
    (if (Utilities|Enum|Equal(Enum) (Variables|Default|GetWinTeam) "")
      (Variables|Default|SetBounces (Utilities|Array|MakeArray 0 0))
      (Utilities|Array|SetArrayElem (Variables|Default|GetPoints) (Variables|Default|GetTempTeam) (+ (Utilities|Array|Get(acopy) (Variables|Default|GetPoints) (Variables|Default|GetTempTeam)) 1))
      (if (>= (Utilities|Array|Get(acopy) (Variables|Default|GetPoints) (Variables|Default|GetTempTeam)) (Variables|Default|GetMaxScore))
        (if (== (Variables|Default|GetTempTeam) 0)
          (Variables|Default|SetWinTeam "Red Team Winns!")
          (else
            (Variables|Default|SetWinTeam "Green Team Winns!")))
        (bind _outactors (Actor|GetAllActorsOfClass "/Game/Blueprints/BP_Win.BP_Win_C"))
        (Development|SetHiddeninGame (Variables|/Game/Blueprints/BP_Win.BP_Win_C|GetWidget (Utilities|Array|Get(acopy) _outactors)) false false)
        (bind _outactors_2 (Actor|GetAllActorsOfClass "/Game/Blueprints/BP_Music.BP_Music_C"))
        (Default|ChangeMusic _outactors_2 2.0)
        (else
          (CallFunction|Reset)
          ;[0.4763 0 1] Changes music to dubstep whe gained point
          (bind _outactors_3 (Actor|GetAllActorsOfClass "/Game/Blueprints/BP_Music.BP_Music_C"))
          (Default|ChangeMusic _outactors_3 1.0)
          (Utilities|FlowControl|Delay 1.0)
          (Default|ChangeMusic _outactors_3 0.0)))
      (else
        (CallFunction|Reset)))
    (else
      (Variables|Default|SetBounces (Utilities|Array|MakeArray 0 0))
      (Utilities|Array|SetArrayElem (Variables|Default|GetBounces) (Variables|Default|GetTempTeam) (+ (Utilities|Array|Get(acopy) (Variables|Default|GetBounces) (Variables|Default|GetTempTeam)) 1)))))

(event Custom|Reset
  (bind _outactors (Actor|GetAllActorsOfClass "/Game/Blueprints/Ball_BP.Ball_BP_C"))
  (Default|ResetBall (Utilities|Array|Get(acopy) _outactors))
  (bind _outactors_2 (Actor|GetAllActorsOfClass "/Game/Blueprints/BP_Mech.BP_Mech_C"))
  (for _array_element _outactors_2
    (Default|Reset _array_element)))

(event EventBeginPlay
  ;[1 1 1] Set camera shit
  (bind _outactors (Actor|GetAllActorsOfClass "/Game/Blueprints/BP_Camera.BP_Camera_C"))
  (for _array_element _outactors
    (Variables|Default|SetPlayCamera _array_element)
    (bind _outactors_2 (Actor|GetAllActorsOfClass "/Game/Blueprints/BP_MenyCamera.BP_MenyCamera_C"))
    (for _array_element_2 _outactors_2
      (bind _output_get (Variables|Default|SetMenyCamera _array_element_2))
      (Variables|Default|SetCurrentCamera _output_get)
      (CallFunction|ResetCamera)
      (bind _returnvalue (UserInterface|CreateWidget "/Game/Blueprints/GameUI.GameUI_C" 0 self))
      (bind _output_get_2 (Variables|Default|SetGameUI _returnvalue))
      (Widget|SetVisibility _returnvalue "Visible")
      (UserInterface|Viewport|AddtoViewport _output_get_2 0)
      (bind _outactors_3 (Actor|GetAllActorsOfClass "/Game/Blueprints/BP_Win.BP_Win_C"))
      (Development|SetHiddeninGame (Variables|/Game/Blueprints/BP_Win.BP_Win_C|GetWidget (Utilities|Array|Get(acopy) _outactors_3)) true false))))

(fn ConstructionScript)

(fn ResetCamera
  (Game|Player|SetViewTargetwithBlend (Game|GetPlayerController 0) (Variables|Default|GetCurrentCamera) 0.0 "VTBlend_Linear" 0.0 false))