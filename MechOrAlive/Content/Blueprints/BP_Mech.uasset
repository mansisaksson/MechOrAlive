(event OnComponentBeginOverlap(Box)
  (params (OtherActor :type Actor%20Object%20Reference) (OtherComp :type Primitive%20Component%20Object%20Reference) (OtherBodyIndex :type Integer) (bFromSweep :type Boolean) (SweepResult :type Hit%20Result%20Structure%20%28by%20ref%29))
  (bind _asball_bp (Utilities|Casting|CastToBall_BP OtherActor))
  (Variables|Default|SetBallRef _asball_bp)
  (Variables|Default|SetCanHitBall true))

(event OnComponentEndOverlap(Box)
  (params (OtherActor :type Actor%20Object%20Reference) (OtherComp :type Primitive%20Component%20Object%20Reference) (OtherBodyIndex :type Integer))
  (Utilities|Casting|CastToBall_BP OtherActor)
  (Variables|Default|SetCanHitBall false))

(event Custom|Reset
  (Transformation|SetActorLocation (Variables|Default|GetInitialPosition) false false))

(event EventBeginPlay
  (Variables|Default|SetInitialPosition (Transformation|GetActorLocation)))

(event EventActorBeginOverlap
  (params (OtherActor :type Actor%20Object%20Reference)))

(event EventTick
  (params (DeltaSeconds :type Float%20%28single-precision%29))
  (bind _returnvalue (Transformation|GetActorLocation))
  (Transformation|SetActorLocation (Math|Vector|MakeVector (.x _returnvalue) 0.0 (.z _returnvalue)) false false))

(event Input|ActionEvents|InputActionSmash
  (params (Key :type Key%20Structure :default "AnyKey"))
  (bind _smash (Variables|Default|GetSmash))
  (:Pressed
    (if (Variables|Default|GetCanHitBall)
      (Default|HitBall (Variables|Default|GetBallRef) (+ (* (Transformation|GetActorForwardVector) 4e+03) "0, 0,1500.000000") self)
      ;[0.5122 0 1] Play Smash Sound
      (Class|FMODAudioComponent|SetParameter _smash "ShotType" 1.0)
      (Class|FMODAudioComponent|Play _smash))))

(event Input|ActionEvents|InputActionLob
  (params (Key :type Key%20Structure :default "AnyKey"))
  (bind _lob (Variables|Default|GetLob))
  (:Pressed
    (if (Variables|Default|GetCanHitBall)
      (Default|HitBall (Variables|Default|GetBallRef) (+ (* (Transformation|GetActorForwardVector) 1e+03) "0, 0,3000.000000") self)
      ;[0.5122 0 1] Play Lob Sound
      (Class|FMODAudioComponent|SetParameter _lob "ShotType" 0.0)
      (Class|FMODAudioComponent|Play _lob))))

(event Input|GamepadEvents|GamepadRightShoulder
  (params (Key :type Key%20Structure :default "AnyKey"))
  (:Pressed
    (bind _outactors (Actor|GetAllActorsOfClass "/Game/Blueprints/Ball_BP.Ball_BP_C"))
    (Utilities|IsValid (Utilities|Array|Get(acopy) _outactors)
      (:Is%20Valid
        (Default|ReleaseBall (Utilities|Array|Get(acopy) _outactors))))))

(event Input|KeyboardEvents|I
  (params (Key :type Key%20Structure :default "AnyKey"))
  (:Pressed
    (bind _outactors (Actor|GetAllActorsOfClass "/Game/Blueprints/Ball_BP.Ball_BP_C"))
    (Utilities|IsValid (Utilities|Array|Get(acopy) _outactors)
      (:Is%20Valid
        (Default|ReleaseBall (Utilities|Array|Get(acopy) _outactors))))))

(fn ConstructionScript)