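; Ball actor for a team-based, volleyball-style game with mechs, handling serve placement, hits and touch counting.
; It starts hidden without gravity, spawns floating above the first mech found, and falls on release.
; HitBall applies impulses while counting consecutive same-team touches, withholding the impulse once the count reaches the limit.
; ResetBall clears touch state and suspends the ball above a mech from the given team.
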(event Custom|ResetBall
  (params (Team :type Integer))
  (Physics|SetEnableGravity (Variables|Default|GetCollider) true)
  (Variables|Default|SetLastTouchedBy 0)
  (Variables|Default|SetNumberOfTouches 0)
  (bind _array_element (Utilities|Array|ForEachLoopwithBreak (Variables|Default|GetCharacters) :!label _label)
    (:LoopBody
      (if (== (Variables|/Game/Blueprints/BP_Mech.BP_Mech_C|GetTeam _array_element) Team)
        (goto _label Break)))
    (:Completed
      (Transformation|SetActorLocation (+ (Transformation|GetActorLocation _array_element) "0, 0,400.000000") false false)
      (Physics|SetEnableGravity (Variables|Default|GetCollider) false))))

(event Custom|SpawnBall
  (params (Team :type Integer))
  (Variables|Default|SetTeamToServe Team)
  (bind _outactors (Actor|GetAllActorsOfClass "/Game/Blueprints/BP_Mech.BP_Mech_C"))
  (bind _output_get (Variables|Default|SetCharacters _outactors))
  (Utilities|IsValid (Utilities|Array|Get(acopy) _output_get)
    (:Is%20Valid
      (Transformation|SetActorLocation (+ (Transformation|GetActorLocation (Utilities|Array|Get(acopy) _output_get)) "0, 0,400.000000") false false)
      (Physics|SetEnableGravity (Variables|Default|GetCollider) false)
      (Rendering|SetActorHiddenInGame false))))

(event Custom|ReleaseBall
  (Physics|SetEnableGravity (Variables|Default|GetCollider) true))

(event EventBeginPlay
  (Rendering|SetActorHiddenInGame true)
  (Physics|SetEnableGravity (Variables|Default|GetCollider) false))

(event EventTick
  (params (DeltaSeconds :type Float%20%28single-precision%29)))

(fn ConstructionScript)

(fn HitBall
  (params (Impulse :type Vector) (Mech :type BP%20Mech%20Object%20Reference))
  (if (== Mech (Variables|Default|GetLastTouchedBy))
    _
    (else
      _))
  (Variables|Default|SetLastTouchedBy Mech)
  (if (== (Variables|Default|GetCurrentTeam) (Variables|/Game/Blueprints/BP_Mech.BP_Mech_C|GetTeam (Variables|Default|GetLastTouchedBy)))
    (bind _output_get (Variables|Default|SetNumberOfTouches (+ (Variables|Default|GetNumberOfTouches) 1)))
    (if (not (>= _output_get 3))
      (Development|PrintString (Utilities|String|ToString(Integer) _output_get))
      (Physics|AddImpulse (Variables|Default|GetCollider) Impulse "None" true :!label _label))
    (else
      (Variables|Default|SetNumberOfTouches 0)
      (Variables|Default|SetCurrentTeam (Variables|/Game/Blueprints/BP_Mech.BP_Mech_C|GetTeam (Variables|Default|GetLastTouchedBy)))
      (goto _label))))